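; Tooltip actor variant whose text turns to face the third-person character's camera while that character is inside its trigger.
; It extends a parent Blueprint, setting a look-at flag on begin overlap if CharacterInBox is valid and clearing it on any end overlap.
; While the flag is set, each Tick casts CharacterInBox to BP_ThirdPersonCharacter and rotates TooltipText toward its FollowCamera using a look-at rotation.
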(event `self.ReceiveTick`
  (params (DeltaSeconds :type "Float (single-precision)"))
  (`parent.ReceiveTick` DeltaSeconds)
  (`self.LookingAtPlayerCamera`))

(event `self.ReceiveBeginPlay`
  (`parent.ReceiveBeginPlay`))

(event `self.ReceiveActorBeginOverlap`
  (params (OtherActor :type "Actor Object Reference"))
  (`parent.ReceiveActorBeginOverlap` OtherActor)
  (`self.CharacterInBox`
    (:`then`
      (set `self.IsLookAtPlayerCamera` true))
    (:`else`)))

(event `self.ReceiveActorEndOverlap`
  (params (OtherActor :type "Actor Object Reference"))
  (`parent.ReceiveActorEndOverlap` OtherActor)
  (set `self.IsLookAtPlayerCamera` false))

(fn `LookingAtPlayerCamera`
  (if (`self.IsLookAtPlayerCamera`)
    (bind _asbp_third_person_character (cast `/Game/Blueprints/Character/BP_ThirdPersonCharacter` (`self.CharacterInBox`)))
    (`SceneComponent.K2_SetWorldRotation` (`self.TooltipText`) (`KismetMathLibrary.FindLookAtRotation` (`SceneComponent.K2_GetComponentLocation` (`self.TooltipText`)) (`SceneComponent.K2_GetComponentLocation` (`/Game/Blueprints/Character/BP_ThirdPersonCharacter.FollowCamera` _asbp_third_person_character))) false false)))

(fn `UserConstructionScript`
  (`parent.UserConstructionScript`))