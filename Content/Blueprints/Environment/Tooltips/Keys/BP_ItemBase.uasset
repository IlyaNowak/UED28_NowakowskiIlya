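; Base item actor with a floating text tooltip and a backpack pickup hook, sized and positioned in the construction script.
; Character overlap shows the tooltip, turns it toward the follow camera each Tick and enables interaction; leaving reverses this.
; Interact passes the character's backpack component to PutIntoBackpack, which is empty here, and returns true on every path.
; AfterUse destroys the actor.
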(event `self.ReceiveTick`
  (params (DeltaSeconds :type "Float (single-precision)"))
  (if (`self.Is Look at Player Camera`)
    (bind _asbp_third_person_character (cast `/Game/Blueprints/Character/BP_ThirdPersonCharacter` (`self.Character in Box`)))
    (`SceneComponent.K2_SetWorldRotation` (`self.TextRender`) (`KismetMathLibrary.FindLookAtRotation` (`SceneComponent.K2_GetComponentLocation` (`self.TextRender`)) (`SceneComponent.K2_GetComponentLocation` (`/Game/Blueprints/Character/BP_ThirdPersonCharacter.FollowCamera` _asbp_third_person_character))) false false)))

(event `self.ReceiveActorBeginOverlap`
  (params (OtherActor :type "Actor Object Reference"))
  (bind _asbp_third_person_character (cast `/Game/Blueprints/Character/BP_ThirdPersonCharacter` OtherActor))
  (set `self.Character in Box` _asbp_third_person_character)
  (`SceneComponent.SetHiddenInGame` (`self.TextRender`) false false)
  (set `self.IsReadyToInteract` true)
  (set `self.Is Look at Player Camera` true))

(event `self.ReceiveActorEndOverlap`
  (params (OtherActor :type "Actor Object Reference"))
  (bind _asbp_third_person_character (cast `/Game/Blueprints/Character/BP_ThirdPersonCharacter` OtherActor))
  (set `self.Character in Box` _asbp_third_person_character)
  (`SceneComponent.SetHiddenInGame` (`self.TextRender`) true false)
  (set `self.IsReadyToInteract` false)
  (set `self.Is Look at Player Camera` false))

(fn `AfterUse`
  (`self.K2_DestroyActor`))

(fn `Interact`
  (returns (Success :type Boolean))
  (if (`self.IsReadyToInteract`)
    (bind _character_in_box (`self.Character in Box`)
      (:`then`
        (bind _returnvalue (`self.GetComponentByClass` _character_in_box "/Game/Blueprints/Components/BP_Backpackomponent.BP_Backpackomponent_C"))
        (`/Engine/EditorBlueprintResources/StandardMacros.IsValid` _returnvalue
          (:`Is Valid`
            (`self.PutIntoBackpack` _returnvalue)
            (return true))
          (:`Is Not Valid`
            (return true))))
      (:`else`
        (return true)))
    (else
      (return true))))

(fn `PutIntoBackpack`
  (params (InBackpack :type "/Game/Blueprints/Components/BP_Backpackomponent Object Reference")))

(fn `UserConstructionScript`
  (`BoxComponent.SetBoxExtent` (`self.ItemCollision`) (`self.Collision Extent`) true)
  (`SceneComponent.K2_SetRelativeLocation` (`self.ItemCollision`) (`KismetMathLibrary.MakeVector` 0.0 0.0 (.z (`self.Collision Extent`))) false false)
  (`SceneComponent.K2_SetRelativeLocation` (`self.TextRender`) (`self.Tooltip Text Location`) false false))