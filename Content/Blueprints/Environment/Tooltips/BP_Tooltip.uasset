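; Tooltip actor that shows a text message in the world while a Character is inside its collision volume.
; The construction script sizes the box from CollisionExtent, lifts it so its base sits at the parent's origin, and applies the configurable text and its location.
; Overlap events store or clear CharacterInBox and toggle text visibility; any Character leaving hides it, even if another remains.
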(event `self.ReceiveActorBeginOverlap`
  (params (OtherActor :type "Actor Object Reference"))
  (bind _ascharacter (cast `Character` OtherActor))
  (set `self.CharacterInBox` _ascharacter)
  (`SceneComponent.SetHiddenInGame` (`self.TooltipText`) false false))

(event `self.ReceiveActorEndOverlap`
  (params (OtherActor :type "Actor Object Reference"))
  (cast `Character` OtherActor)
  (set `self.CharacterInBox` null)
  (`SceneComponent.SetHiddenInGame` (`self.TooltipText`) true false))

(fn `UserConstructionScript`
  (`BoxComponent.SetBoxExtent` (`self.TooltipCollision`) (`self.CollisionExtent`) true)
  (`SceneComponent.K2_SetRelativeLocation` (`self.TooltipCollision`) (`KismetMathLibrary.MakeVector` 0.0 0.0 (.z (`self.CollisionExtent`))) false false)
  (`SceneComponent.K2_SetRelativeLocation` (`self.TooltipText`) (`self.TooltipTextLocation`) false false)
  (`TextRenderComponent.K2_SetText` (`self.TooltipText`) (`self.TooltipTextMassage`)))