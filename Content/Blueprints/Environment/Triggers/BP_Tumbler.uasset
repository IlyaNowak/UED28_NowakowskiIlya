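; BP_Tumbler is an interactable toggle switch that flips the lock state of its linked doors.
; Interact plays or reverses a timeline that slides the stick along local Y, ignoring animation requests mid-move, but switches the door locks on every call.
; The construction script offsets the stick for the initial on state, and overlap shows or hides a text prompt.
; Tick prints the stick's location as debug output.
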(event `self.ReceiveTick`
  (params (DeltaSeconds :type "Float (single-precision)"))
  (`KismetSystemLibrary.PrintString` (`KismetStringLibrary.Conv_VectorToString` (`SceneComponent.RelativeLocation` (`self.TumblerStickMesh`))) true true (struct :`G` 0.66 :`B` 1.0 :`A` 1.0) 0.0))

(event `self.ReceiveActorBeginOverlap`
  (params (OtherActor :type "Actor Object Reference"))
  (set `self.OverlappedActor` OtherActor)
  (`SceneComponent.SetVisibility` (`self.TextRender`) true false))

(event `self.ReceiveActorEndOverlap`
  (params (OtherActor :type "Actor Object Reference"))
  (set `self.OverlappedActor` null)
  (`SceneComponent.SetVisibility` (`self.TextRender`) false false))

(event `TumblerOn`
  (if (not (`self.InProgress`))
    (if (not (`self.IsTumblerOn`))
      (bind (_direction _tumblertimeline) (`Timeline|Timeline` :!via `PlayFromStart` :!label _label)
        (:`Update`
          (set `self.InProgress` true)
          (`SceneComponent.K2_SetRelativeLocation` (`self.TumblerStickMesh`) (`KismetMathLibrary.MakeVector` 0.0 (`KismetMathLibrary.Lerp` -5.0 (/ (`self.MaxTumblerOffset`) 2.0) _tumblertimeline)) false false))
        (:`Finished`
          (set `self.InProgress` false)
          (switch `ETimelineDirection` _direction
            (:`Forward`
              (set `self.IsTumblerOn` true))
            (:`Backward`
              (set `self.IsTumblerOn` false))))))))

(event `TumblerOff`
  (if (not (`self.InProgress`))
    (if (`self.IsTumblerOn`)
      (goto _label :!via `ReverseFromEnd`))))

(fn `Interact`
  (returns (Success :type Boolean))
  (if (`self.IsTumblerOn`)
    (`self.TumblerOff`)
    (else
      (`self.TumblerOn`)))
  (`self.SwitchDoorsLock`)
  (return true))

(fn `SwitchDoorsLock`
  (for _array_element (`self.DoorsToLockSwitchTumbler`)
    (`/Game/Blueprints/Environment/Doors/BP_Door_WithLock.SwitchLock` _array_element)))

(fn `UserConstructionScript`
  (`SceneComponent.K2_AddRelativeLocation` (`self.TumblerStickMesh`) (`KismetMathLibrary.MakeVector` 0.0 (`KismetMathLibrary.SelectFloat` (`self.MaxTumblerOffset`) 0.0 (`self.IsTumblerOn`))) false false))