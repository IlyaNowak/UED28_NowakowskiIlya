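; BP_Door_WithLock is a child door actor that opens only when unlocked, with a point light showing red or green for lock state.
; Interact toggles an unlocked door; when locked, it checks the overlapped actor's backpack quest items against NeedKeys.
; Having every key unlocks it without opening or consuming keys; otherwise an indicator shows the missing count.
; Lock only works on doors without required keys, while SwitchLock toggles regardless.
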(event `self.OpenDoor`
  (if (not (`self.IsDoorLocked`))
    (`parent.OpenDoor`)))

(event `self.CloseDoor`
  (`parent.CloseDoor`))

(fn `Interact`
  (returns (Success :type Boolean))
  (locals (L_ItemInrement :type Integer) (L_ItemName :type Name))
  (bind _l_iteminrement (`local.L_ItemInrement`))
  (bind _returnvalue (`KismetArrayLibrary.Array_Length` (`self.NeedKeys`)))
  (if (`self.IsReadyToInteract`)
    (if (not (`self.IsDoorLocked`))
      (if (`self.IsDoorOpen`)
        (`self.CloseDoor`)
        (else
          (`self.OpenDoor`)))
      (return true)
      (elif (`KismetArrayLibrary.Array_IsValidIndex` (`self.NeedKeys`))
        (bind _overlappedactor (`self.OverlappedActor`)
          (:`then`
            (bind _returnvalue_2 (`self.GetComponentByClass` _overlappedactor "/Game/Blueprints/Components/BP_Backpackomponent.BP_Backpackomponent_C"))
            (`/Engine/EditorBlueprintResources/StandardMacros.IsValid` _returnvalue_2
              (:`Is Valid`
                (set `self.L_Backpack` _returnvalue_2)
                (for _array_element (`self.NeedKeys`)
                  (set `local.L_ItemName` _array_element)
                  (if (`BlueprintSetLibrary.Set_Contains` (`/Game/Blueprints/Components/BP_Backpackomponent.QuestItems` (`self.L_Backpack`)) (`local.L_ItemName`))
                    (`/Engine/EditorBlueprintResources/StandardMacros.IncrementInt` (`local.L_ItemInrement`))))
                (if (== _l_iteminrement _returnvalue)
                  (`self.UnLock`)
                  (else
                    (`TextRenderComponent.K2_SetText` (`self.KeysNeedIndicator`) (`KismetTextLibrary.Conv_IntToText` (- _returnvalue _l_iteminrement)))
                    (return true))))
              (:`Is Not Valid`
                (return true))))
          (:`else`
            (return true)))
        (else
          (return true))))
    (else
      (return false))))

(fn `Lock`
  (if (not (`KismetArrayLibrary.Array_IsValidIndex` (`self.NeedKeys`)))
    (set `self.IsDoorLocked` true)
    (`self.UpdateDoorLockIndication`)))

(fn `SwitchLock`
  (set `self.IsDoorLocked` (not (`self.IsDoorLocked`)))
  (`self.UpdateDoorLockIndication`))

(fn `UnLock`
  (set `self.IsDoorLocked` false)
  (`self.UpdateDoorLockIndication`))

(fn `UpdateDoorLockIndication`
  (`LightComponent.SetLightColor` (`self.PointLightLockIndicator`) (`KismetMathLibrary.SelectColor` (struct :`R` 1.0 :`B` 0.035352 :`A` 1.0) (struct :`R` 0.288836 :`G` 1.0 :`A` 1.0) (`self.IsDoorLocked`)) true))

(fn `UserConstructionScript`
  (`parent.UserConstructionScript`)
  (`self.UpdateDoorLockIndication`))